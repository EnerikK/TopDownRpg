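; BP_FlamePillar is a flame pillar actor that continuously varies the intensity of its fire light.
; From BeginPlay, it randomly plays one of two intensity timelines and picks again whenever one finishes, forming an endless loop.
; Each timeline update passes its curve value to ScaleFlameIntensity, which multiplies it by BaseIntensity and applies it to FireLight, without using Tick.
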(event `self.ReceiveBeginPlay`
  (`self.ChooseTimeLine`))

(event `ChooseTimeLine`
  (switch `int` (`KismetMathLibrary.RandomIntegerInRange` 0 1)
    (:`Default`
      (`self.StartTimeLine2` :!label _label))
    (:`0`
      (`self.StartTimeline1`))
    (:`1`
      (goto _label))))

(event `StartTimeline1`
  (bind (_direction _flameintenisty) (`Timeline|FlameIntensity1` :!via `PlayFromStart`)
    (:`Update`
      (`self.ScaleFlameIntensity` _flameintenisty))
    (:`Finished`
      (`self.ChooseTimeLine`))))

(event `StartTimeLine2`
  (bind (_direction _flameintensity) (`Timeline|FlameIntensity2` :!via `PlayFromStart`)
    (:`Update`
      (`self.ScaleFlameIntensity` _flameintensity))
    (:`Finished`
      (`self.ChooseTimeLine`))))

(fn `ScaleFlameIntensity`
  (params (Intensity :type "Float (double-precision)"))
  (`LightComponent.SetIntensity` (`self.FireLight`) (* Intensity (`self.BaseIntensity`))))

(fn `UserConstructionScript`)