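; BP_FadeActor is a static mesh actor that fades out and back in, triggering both itself on BeginPlay, one second apart.
; Construction caches original materials and builds dynamic instances from MaterialInstances.
; FadeOut applies these and plays a timeline driving their "Fade" parameter, which FadeIn reverses.
; On finish, full fade value restores original materials and blocks the Visibility channel, while zero ignores that channel.
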(event `self.ReceiveBeginPlay`
  (`self.FadeOut`)
  (`KismetSystemLibrary.Delay` 1.0)
  (`self.FadeIn`))

(event `/Game/Blueprints/Actor/FadeActor/BI_FadeInterface.FadeOut`
  (`self.SetMaterialToDyamicInstances`)
  (bind (_direction _fade) (`Timeline|Timeline` :!label _label)
    (:`Update`
      (for _array_element (`self.DynamicMaterialInstances`)
        (`MaterialInstanceDynamic.SetScalarParameterValue` _array_element "Fade" _fade)))
    (:`Finished`
      (`self.FadeFinished` _fade _fade))))

(event `/Game/Blueprints/Actor/FadeActor/BI_FadeInterface.FadeIn`
  (goto _label :!via `Reverse`))

(fn `FadeFinished`
  (params (A :type "Float (double-precision)") (A2 :type "Float (double-precision)"))
  (if (>= A2 1.0)
    (`self.ResetMaterials`)
    (`PrimitiveComponent.SetCollisionResponseToChannel` (`self.StaticMesh`) "ECC_Visibility" "ECR_Block")
    (elif (<= A 0.0)
      (`PrimitiveComponent.SetCollisionResponseToChannel` (`self.StaticMesh`) "ECC_Visibility" "ECR_Ignore"))))

(fn `ResetMaterials`
  (for (_array_element _array_index) (`self.OriginalMaterials`)
    (`PrimitiveComponent.SetMaterial` (`self.StaticMesh`) _array_index _array_element)))

(fn `SetMaterialToDyamicInstances`
  (for (_array_element _array_index) (`self.DynamicMaterialInstances`)
    (`PrimitiveComponent.SetMaterial` (`self.StaticMesh`) _array_index _array_element)))

(fn `UserConstructionScript`
  (`KismetArrayLibrary.Array_Clear` (`self.DynamicMaterialInstances`))
  (set `self.OriginalMaterials` (`MeshComponent.GetMaterials` (`self.StaticMesh`)))
  (for _array_element (`self.MaterialInstances`)
    (bind _returnvalue (`KismetMaterialLibrary.CreateDynamicMaterialInstance` _array_element))
    (`KismetArrayLibrary.Array_AddUnique` (`self.DynamicMaterialInstances`) _returnvalue)))