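; Firebolt gameplay ability that fires projectiles from the weapon socket toward the target under the mouse.
; On activation it commits, takes the hit location and actor from cursor target data, turns the avatar toward it and plays the cast montage.
; A montage gameplay event triggers the spawn, passing the hit actor as homing target.
; The ability ends when the montage completes, blends out or is interrupted or cancelled.
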(event `self.K2_ActivateAbility`
  (`self.K2_CommitAbility`)
  (bind (_asynctaskproxy _datahandle) (`TargetDataUnderMouse.CreateTargetDataUnderMouse`)
    (:`ValidData`
      (bind (_bblockinghit _binitialoverlap _time _distance _location _impactpoint _normal _impactnormal _physmat _hitactor) (`GameplayStatics.BreakHitResult` (`AbilitySystemBlueprintLibrary.GetHitResultFromTargetData` _datahandle)))
      (set `self.MouseHitActor` _hitactor)
      (bind _output_get (set `self.ProjectileTargetLocation` _location))
      (message `CombatInterface.UpdateFacingTarget` (`self.GetAvatarActorFromActorInfo`) _output_get)
      (`AbilityTask_PlayMontageAndWait.CreatePlayMontageAndWaitProxy` "None" "/Game/Assets/Characters/Aura/Animations/Abilities/Montage_FireBolt.Montage_FireBolt" 1.0 "None" false
        (:`then`
          (`AbilityTask_WaitGameplayEvent.WaitGameplayEvent` (struct :`TagName` "Event.Montage.Firebolt") null
            (:`EventReceived`
              (`self.SpawnProjectiles` (`self.ProjectileTargetLocation`) (`BlueprintGameplayTagLibrary.MakeLiteralGameplayTag` (struct :`TagName` "CombatSocket.Weapon")) false 0.0 (`self.MouseHitActor`)))))
        (:`OnCompleted`
          (`self.K2_EndAbility` :!label _label))
        (:`OnBlendOut`
          (goto _label))
        (:`OnInterrupted`
          (goto _label))
        (:`OnCancelled`
          (goto _label))))))

(event `self.K2_OnEndAbility`
  (params (bWasCancelled :type Boolean)))