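; Channeled lightning Gameplay Ability: a beam from the caster's weapon to the cursor target that chains to additional targets.
; A montage event locks movement, adds looping GameplayCues and starts a timer that commits cost and applies lightning damage to all targets.
; Input release (padded to a minimum cast time on authority), failed cost or primary target death removes cues, applies a final damage effect and commits cooldown.
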(event `self.PrimaryTargetDie`
  (params (DeadActor :type "Actor Object Reference"))
  (`GameplayCueFunctionLibrary.RemoveGameplayCueOnActor` DeadActor (struct :`TagName` "GameplayCue.ElectroLoop") (`self.FirstTargetCueParams`))
  (`self.ClearTimer&AbilityEnd`))

(event `self.AdditionalTargetDied`
  (params (DeadActor :type "Actor Object Reference"))
  (`self.RemoveLoopFromAdditionalTargets` DeadActor)
  (`KismetArrayLibrary.Array_RemoveItem` (`self.AdditionalTargets`) DeadActor))

(event `self.K2_ActivateAbility`
  (`self.ImplentsInterface?`)
  ;[1 1 1] Store mouse Data
  (bind (_asynctaskproxy _datahandle) (`TargetDataUnderMouse.CreateTargetDataUnderMouse`)
    (:`ValidData`
      (`self.StoreMouseDataInfo` (`AbilitySystemBlueprintLibrary.GetHitResultFromTargetData` _datahandle))
      (`self.StoreOwnerVariables`)
      (`|ExecutionSequence`
        (:`then_0`
          (set `PlayerController.bShowMouseCursor` false (`self.OwnerPlayerController`))
          (`self.UpdateFacingTarget`)
          (`self.K2_ExecuteGameplayCue` (struct :`TagName` "GameplayCue.ElectroShock"))
          (`AbilityTask_PlayMontageAndWait.CreatePlayMontageAndWaitProxy` "None" (`self.Montage_Electro`) 1.0 "None" false
            (:`then`
              (`AbilityTask_WaitGameplayEvent.WaitGameplayEvent` (struct :`TagName` "Event.Montage.Electro") null
                (:`EventReceived`
                  (`self.ShockLooping`)
                  (`self.SpawnElectro`)
                  (bind _returnvalue (`KismetSystemLibrary.K2_SetTimerDelegate` (delegate `DamageAndCost`) (`self.DamageDeltaTime`) true))
                  (set `self.DamageAndCostTimer` _returnvalue))))))
        (:`then_1`
          (bind (_asynctaskproxy_2 _timeheld) (`AbilityTask_WaitInputRelease.WaitInputRelease` false)
            (:`OnRelease`
              (set `self.Time Held` _timeheld)
              (if (< (`self.Time Held`) (`self.MinSpellTime`))
                (`self.K2_HasAuthority`
                  (:`True`
                    (`KismetSystemLibrary.Delay` (- (`self.MinSpellTime`) (`self.Time Held`)))
                    (`self.ClearTimer&AbilityEnd` :!label _label))
                  (:`False`
                    (`self.PrepareToEnd`)))
                (else
                  (goto _label))))))))))

(event `DamageAndCost`
  (bind _returnvalue (`self.K2_CommitAbilityCost` false))
  (if _returnvalue
    (`self.ApplyDamage`)
    (else
      (`self.ClearTimer&AbilityEnd`))))

(fn `AddElectroToAdditionalTargets`
  (params (AdditionalTarget :type "Actor Object Reference"))
  (locals (TargetActor :type "Actor Object Reference"))
  (bind _targetactor (`local.TargetActor`))
  (bind _returnvalue (`AbilitySystemBlueprintLibrary.MakeGameplayCueParameters` 0.0 0.0 (struct) (struct) (struct) (struct) (struct) (`Actor.K2_GetActorLocation` _targetactor) (0.0 0.0 0.0) null null _targetactor null 1 1 (`Actor.RootComponent` (`self.MouseHitActor`))))
  (set `local.TargetActor` AdditionalTarget)
  (`BlueprintMapLibrary.Map_Add` (`self.AdditionalActorsToCueParams`) (`local.TargetActor`) _returnvalue)
  (`GameplayCueFunctionLibrary.AddGameplayCueOnActor` (`local.TargetActor`) (struct :`TagName` "GameplayCue.ElectroLoop") _returnvalue))

(fn `ApplyDamage`
  (`self.ApplyDamageSingleTarget` (`self.MouseHitActor`))
  (for _array_element (`self.AdditionalTargets`)
    (`self.ApplyDamageSingleTarget` _array_element)))

(fn `ApplyDamageSingleTarget`
  (params (Actor :type "Actor Object Reference"))
  (locals (ASC :type "AbilitySystemComponent Object Reference"))
  (bind _returnvalue (`AbilitySystemBlueprintLibrary.GetAbilitySystemComponent` (`self.DamagedTarget`)))
  (bind _output_get (set `self.DamagedTarget` Actor))
  (`/Engine/EditorBlueprintResources/StandardMacros.IsValid` _output_get
    (:`Is Valid`
      (bind _output_get_2 (set `local.ASC` (`self.GetAbilitySystemComponentFromActorInfo`)))
      (`/Engine/EditorBlueprintResources/StandardMacros.IsValid` _output_get_2
        (:`Is Valid`
          (bind _returnvalue_2 (`AbilitySystemBlueprintLibrary.AssignTagSetByCallerMagnitude` (`AbilitySystemComponent.MakeOutgoingSpec` (`local.ASC`) (`self.DamageEffectClass`) (`KismetMathLibrary.Conv_IntToDouble` (`self.GetAbilityLevel`)) (`AbilitySystemComponent.MakeEffectContext` (`local.ASC`))) (struct :`TagName` "Damage.Lightning") (`self.GetDamageAtLevel`)))
          (`/Engine/EditorBlueprintResources/StandardMacros.IsValid` _returnvalue
            (:`Is Valid`
              (`AbilitySystemComponent.BP_ApplyGameplayEffectSpecToSelf` _returnvalue _returnvalue_2))))))))

(fn `ClearTimer&AbilityEnd`
  (`KismetSystemLibrary.K2_ClearAndInvalidateTimerHandle` (`self.DamageAndCostTimer`))
  (`self.PrepareToEnd`)
  (`self.K2_CommitAbilityCooldown` false)
  (`KismetArrayLibrary.Array_Clear` (`self.AdditionalTargets`))
  (`BlueprintMapLibrary.Map_Clear` (`self.AdditionalActorsToCueParams`))
  (set `self.MouseHitActor` null)
  (set `self.ImplementsInterface?` false)
  (set `self.Time Held` 0.0)
  (`self.K2_EndAbility`))

(fn `ImplentsInterface?`
  (if (not (`KismetSystemLibrary.DoesImplementInterface` (`self.GetAvatarActorFromActorInfo`) "/Script/Aura.CombatInterface"))
    (`self.K2_EndAbility`)))

(fn `PrepareToEnd`
  (bind _mousehitactor (`self.MouseHitActor`))
  (set `PlayerController.bShowMouseCursor` true (`self.OwnerPlayerController`))
  (message `CombatInterface.SetInShockLoop` (`self.GetAvatarActorFromActorInfo`) false)
  (`CharacterMovementComponent.SetMovementMode` (`Character.CharacterMovement` (`self.OwnerCharacter`)) "MOVE_Walking" 0)
  (if (`self.ImplementsInterface?`)
    (`GameplayCueFunctionLibrary.RemoveGameplayCueOnActor` _mousehitactor (struct :`TagName` "GameplayCue.ElectroLoop") (`self.FirstTargetCueParams`))
    (`self.K2_HasAuthority`
      (:`True`
        (`AuraAbilitySystemLibrary.ApplyDamageEffect` (`self.MakeDamageEffectParamsFromClassDefaults` _mousehitactor)))
      (:`False`
        _))
    (for _array_element (`self.AdditionalTargets`)
      (bind (_value _returnvalue) (`BlueprintMapLibrary.Map_Find` (`self.AdditionalActorsToCueParams`) _array_element))
      (if _returnvalue
        (`GameplayCueFunctionLibrary.RemoveGameplayCueOnActor` _array_element (struct :`TagName` "GameplayCue.ElectroLoop") _value)
        (`self.K2_HasAuthority`
          (:`True`
            (`AuraAbilitySystemLibrary.ApplyDamageEffect` (`self.MakeDamageEffectParamsFromClassDefaults` _array_element))))))
    (else
      (`GameplayCueFunctionLibrary.RemoveGameplayCueOnActor` (`self.GetAvatarActorFromActorInfo`) (struct :`TagName` "GameplayCue.ElectroLoop") (`self.FirstTargetCueParams`)))))

(fn `RemoveLoopFromAdditionalTargets`
  (params (AdditionalTargets :type "Actor Object Reference"))
  (bind (_value _returnvalue) (`BlueprintMapLibrary.Map_Find` (`self.AdditionalActorsToCueParams`) (`local.AdditionalTargets`)))
  (set `self.Additional Targets` AdditionalTargets)
  (if _returnvalue
    (`GameplayCueFunctionLibrary.RemoveGameplayCueOnActor` (`local.AdditionalTargets`) (struct :`TagName` "GameplayCue.ElectroLoop") _value)))

(fn `ShockLooping`
  (message `CombatInterface.SetInShockLoop` (`self.GetAvatarActorFromActorInfo`) true)
  (`CharacterMovementComponent.DisableMovement` (`Character.CharacterMovement` (`self.OwnerCharacter`))))

(fn `SpawnElectro`
  (`self.TraceFirstTarget` (`self.MouseHitLocation`))
  (bind _returnvalue (message `CombatInterface.GetWeapon` (`self.OwnerCharacter`)))
  (set `self.FirstTargetCueParams` (`AbilitySystemBlueprintLibrary.MakeGameplayCueParameters` 0.0 0.0 (struct) (struct) (struct) (struct) (struct) (`self.MouseHitLocation`) (0.0 0.0 0.0) null null (`self.MouseHitActor`) null 1 1 _returnvalue))
  ;[1 1 1] IsMouseHitActor an Enemy?
  (bind _output_get (set `self.ImplementsInterface?` (`KismetSystemLibrary.DoesImplementInterface` (`self.MouseHitActor`) "/Script/Aura.CombatInterface")))
  (if _output_get
    (set `self.CueTarget` (`self.MouseHitActor`))
    (else
      (set `self.CueTarget` (`self.GetAvatarActorFromActorInfo`))))
  (`GameplayCueFunctionLibrary.AddGameplayCueOnActor` (`self.CueTarget`) (struct :`TagName` "GameplayCue.ElectroLoop") (`self.FirstTargetCueParams`))
  (if (`self.ImplementsInterface?`)
    (bind _outadditionaltargets (`self.StoreAdditionalTargets`))
    (bind _output_get_2 (set `self.AdditionalTargets` _outadditionaltargets))
    (for _array_element _output_get_2
      (`self.AddElectroToAdditionalTargets` _array_element))))

(fn `UpdateFacingTarget`
  (message `CombatInterface.UpdateFacingTarget` (`self.GetAvatarActorFromActorInfo`) (`self.MouseHitLocation`)))