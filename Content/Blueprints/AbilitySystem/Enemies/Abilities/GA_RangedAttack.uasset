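; Enemy gameplay ability that fires a projectile at the avatar's combat target during a ranged attack animation.
; On activation it faces the avatar toward the target and plays a random tagged attack montage.
; A gameplay event matching the montage's tag times the shot, spawning the projectile toward the target's location at that moment.
; The socket location queried then is not passed on, and the graph never ends the ability.
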(event `self.K2_ActivateAbility`
  (bind _returnvalue (`self.GetAvatarActorFromActorInfo`))
  (bind _returnvalue_2 (`self.GetAvatarActorFromActorInfo`))
  (bind _returnvalue_3 (message `EnemyInterface.GetCombatTarget` _returnvalue))
  (message `CombatInterface.UpdateFacingTarget` _returnvalue (`Actor.K2_GetActorLocation` _returnvalue_3))
  (bind _returnvalue_4 (message `CombatInterface.GetAttackMontages` (`self.GetAvatarActorFromActorInfo`)))
  (bind _output_get (set `self.TaggedMontage` (`self.GetRandomTaggedMontageFromArray` _returnvalue_4)))
  (bind (_montage _gameplaytag) (break `TaggedMontage` _output_get))
  (`AbilityTask_PlayMontageAndWait.CreatePlayMontageAndWaitProxy` "None" _montage
    (:`then`
      (`AbilityTask_WaitGameplayEvent.WaitGameplayEvent` _gameplaytag null
        (:`EventReceived`
          (message `CombatInterface.GetCombatSocketLocation` _returnvalue_2 _gameplaytag)
          (bind _returnvalue_5 (message `EnemyInterface.GetCombatTarget` _returnvalue_2))
          (`self.SpawnProjectile` (`Actor.K2_GetActorLocation` _returnvalue_5)))))))