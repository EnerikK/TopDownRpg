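; Arcane Shards gameplay ability: shows a magic circle, then on input press erupts damaging shards around the targeted point under the mouse.
; A temporary BP_PointCollection supplies ground points, their count set by ability level up to a cap.
; After a montage event, a looping timer triggers one shard cue per point, applying radial damage to nearby live players except the caster.
; Cost commits at the first shard, cooldown after the last.
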(event `self.K2_ActivateAbility`
  (`self.K2_CheckAbilityCost`)
  (`|ExecutionSequence`
    (:`then_0`
      (message `PlayerInterface.ShowMagicCircle` (`self.GetAvatarActorFromActorInfo`) null))
    (:`then_1`
      (`AbilityTask_WaitInputPress.WaitInputPress` false
        (:`OnPress`
          ;[1 1 1] GetTarget Data
          (bind (_asynctaskproxy _datahandle) (`TargetDataUnderMouse.CreateTargetDataUnderMouse`)
            (:`ValidData`
              (bind _output_get (set `self.MouseHitLocation` (`.ImpactPoint` (`GameplayStatics.BreakHitResult` (`AbilitySystemBlueprintLibrary.GetHitResultFromTargetData` _datahandle)))))
              ;[1 1 1] SpawnPointCollectionAndGetGroundPoints
              (bind _returnvalue (`|SpawnActorFromClass` "/Game/Blueprints/AbilitySystem/Aura/Abilities/Arcane/ArcaneShards/BP_PointCollection.BP_PointCollection_C" (`KismetMathLibrary.MakeTransform` _output_get) "AlwaysSpawn" "MultiplyWithRoot" null null))
              (bind _output_get_2 (set `self.PointCollection` _returnvalue))
              (bind _output_get_3 (set `self.NumShards` (`KismetMathLibrary.Min` (`self.MaxNumShards`) (`self.GetAbilityLevel`))))
              (set `self.GroundPoints` (`PointCollection.GetGroundPoints` _output_get_2 (`self.MouseHitLocation`) _output_get_3 0.0))
              ;[1 1 1] UpdateFace Target
              (message `CombatInterface.UpdateFacingTarget` (`self.GetAvatarActorFromActorInfo`) (`self.MouseHitLocation`))
              ;[1 1 1] PlayMontage and wait for event
              (`AbilityTask_PlayMontageAndWait.CreatePlayMontageAndWaitProxy` "None" "/Game/Assets/Characters/Aura/Animations/Abilities/Montage_ArcaneShard.Montage_ArcaneShard" 1.0 "None" false
                (:`then`
                  (`AbilityTask_WaitGameplayEvent.WaitGameplayEvent` (struct :`TagName` "Event.Montage.ArcaneShards") null true
                    (:`EventReceived`
                      (bind _returnvalue_2 (`KismetSystemLibrary.K2_SetTimerDelegate` (delegate `SpawnParticle`) (`self.ParticleSpawnDeltaTime`) true))
                      (set `self.ParticleSpawnTimer` _returnvalue_2)
                      (message `PlayerInterface.HideMagicCircle` (`self.GetAvatarActorFromActorInfo`) null)
                      (`self.SpawnParticle`)
                      (`self.K2_CommitAbilityCost` false))))))))))))

(event `SpawnParticle`
  (if (< (`self.Count`) (`self.NumShards`))
    (`self.StoreShardLocation`)
    (`self.StorePlayersToDamage`)
    (for _array_element (`self.PlayersToDamage`)
      (`self.RadialDamageToPlayer` _array_element))
    (`/Engine/EditorBlueprintResources/StandardMacros.IncrementInt` (`self.Count`)
      (:`  `
        (`self.K2_ExecuteGameplayCueWithParams` (struct :`TagName` "GameplayCue.ArcaneShards") (`AbilitySystemBlueprintLibrary.MakeGameplayCueParameters` 0.0 0.0 (struct) (struct) (struct) (struct) (struct) (`self.ShardSpawnLocation`)))))
    (else
      (`KismetSystemLibrary.K2_ClearAndInvalidateTimerHandle` (`self.ParticleSpawnTimer`))
      (`Actor.K2_DestroyActor` (`self.PointCollection`))
      (`self.K2_CommitAbilityCooldown` false)
      (`self.K2_EndAbility`))))

(fn `RadialDamageToPlayer`
  (params (TargetActor :type "Actor Object Reference"))
  (`AuraAbilitySystemLibrary.ApplyDamageEffect` (`self.MakeDamageEffectParamsFromClassDefaults` TargetActor (`self.ShardSpawnLocation`))))

(fn `StorePlayersToDamage`
  (bind _returnvalue (`self.GetAvatarActorFromActorInfo`))
  (bind _outoverlappingactors (`AuraAbilitySystemLibrary.GetLivePlayersWithinRadius` _returnvalue (`|MakeArray` _returnvalue) (`self.RadialDamageOuterRadius`) (`self.ShardSpawnLocation`)))
  (set `self.PlayersToDamage` _outoverlappingactors))

(fn `StoreShardLocation`
  (set `self.ShardSpawnLocation` (`SceneComponent.K2_GetComponentLocation` (`|GetArrayItem` (`self.GroundPoints`) (`self.Count`)))))