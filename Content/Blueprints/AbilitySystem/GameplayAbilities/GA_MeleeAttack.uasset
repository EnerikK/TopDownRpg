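; Gameplay ability for a melee attack: the avatar faces its combat target, plays a random attack montage and damages nearby hostiles.
; Montages come from the avatar through combat interface messages, each paired with a gameplay tag.
; That tag's gameplay event triggers a small radius query at the matching combat socket, damaging each live non-friend found.
; The ability ends after the hit event, when the montage finishes or is interrupted, or immediately without montages.
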(event `self.K2_ActivateAbility`
  (bind _returnvalue (`self.GetAvatarActorFromActorInfo`))
  (bind _returnvalue_2 (`self.GetAvatarActorFromActorInfo`))
  (bind _returnvalue_3 (message `EnemyInterface.GetCombatTarget` _returnvalue))
  (bind _ascombat_interface (cast `CombatInterface` _returnvalue))
  (`CombatInterface.UpdateFacingTarget` _ascombat_interface (`Actor.K2_GetActorLocation` _returnvalue_3))
  (bind _returnvalue_4 (message `CombatInterface.GetAttackMontages` (`self.GetAvatarActorFromActorInfo`)))
  (bind _returnvalue_5 (`KismetArrayLibrary.Array_Length` _returnvalue_4))
  (bind _output_get (set `self.TaggedMontage` (`|GetArrayItem` _returnvalue_4 (`KismetMathLibrary.RandomIntegerInRange` 0 (- _returnvalue_5 1)))))
  (if (> _returnvalue_5 0)
    (bind (_montage _gameplaytag) (break `TaggedMontage` _output_get))
    (`AbilityTask_PlayMontageAndWait.CreatePlayMontageAndWaitProxy` "None" _montage 1.0 "None" false
      (:`then`
        (`AbilityTask_WaitGameplayEvent.WaitGameplayEvent` _gameplaytag null
          (:`EventReceived`
            (bind _returnvalue_6 (message `CombatInterface.GetCombatSocketLocation` _returnvalue_2 _gameplaytag))
            (bind _outoverlappingactors (`AuraAbilitySystemLibrary.GetLivePlayersWithinRadius` _returnvalue_2 (`|MakeArray` _returnvalue_2) 45.0 _returnvalue_6))
            (for _array_element _outoverlappingactors
              (if (`AuraAbilitySystemLibrary.IsNotFriend` (`self.GetAvatarActorFromActorInfo`) _array_element)
                (`self.CauseDamage` _array_element)))
            (`self.K2_EndAbility`))))
      (:`OnCompleted`
        (`self.K2_EndAbility` :!label _label))
      (:`OnInterrupted`
        (goto _label))
      (:`OnCancelled`
        (goto _label)))
    (else
      (`self.K2_EndAbility`))))