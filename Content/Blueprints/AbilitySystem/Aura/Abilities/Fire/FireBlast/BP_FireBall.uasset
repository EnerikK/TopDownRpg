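; BP_FireBall is the Fire Blast projectile that flies out, boomerangs back to its ReturnToActor and explodes.
; On the authority, one timeline lerps it forward to an apex, then a second lerps it toward that actor's current location.
; Within ExplodeDistance it calls OnHit, applies radial damage to nearby live players except its owner, with upward-angled knockback and death impulse, then destroys itself.
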(event `self.StartOutGoingTimeLine`
  (bind _explosiondamageparams (`self.ExplosionDamageParams`))
  (bind (_returnvalue_roll _returnvalue_pitch _returnvalue_yaw) (`KismetMathLibrary.BreakRotator` (`KismetMathLibrary.MakeRotFromX` (`self.KnockBackDirection`))))
  (bind _array (`|MakeArray` (`self.GetOwner`)))
  (`/Engine/EditorBlueprintResources/ActorMacros.Switch Has Authority`
    (:`Authority`
      ;[1 0.6978 0] Store The Initial Location and the end(ApexLocation)
      (set `self.InitialLocation` (`self.K2_GetActorLocation`))
      (set `self.ApexLocation` (+ (`self.InitialLocation`) (* (`self.GetActorForwardVector`) (`self.TravelDistance`))))
      ;[1 1 1] GoingOut
      (bind (_direction _outgoingtrack) (`Timeline|OutGoingTimeLine`)
        (:`Update`
          (`self.K2_SetActorLocation` (`KismetMathLibrary.VLerp` (`self.InitialLocation`) (`self.ApexLocation`) _outgoingtrack)))
        (:`Finished`
          ;[1 1 1] ComingBack
          (bind _returntoactor (`self.ReturnToActor`)
            (:`then`
              (bind (_direction_2 _newtrack_0) (`Timeline|Return`)
                (:`Update`
                  (`self.K2_SetActorLocation` (`KismetMathLibrary.VLerp` (`self.ApexLocation`) (`self.K2_GetActorLocation` _returntoactor) _newtrack_0))
                  (if (`self.IsWithingDistance`)
                    (`self.OnHit`)
                    (`KismetArrayLibrary.Array_Add` _array self)
                    (bind _outoverlappingactors (`AuraAbilitySystemLibrary.GetLivePlayersWithinRadius` self _array 200.0 (`self.K2_GetActorLocation`)))
                    (`AuraAbilitySystemLibrary.SetIsRadialDamageEffectParam` (`self.ExplosionDamageParams`) true 50.0 200.0 (`self.K2_GetActorLocation`))
                    (for _array_element _outoverlappingactors
                      (`AuraAbilitySystemLibrary.SetTargetEffectParamsASC` (`self.ExplosionDamageParams`) (`AbilitySystemBlueprintLibrary.GetAbilitySystemComponent` _array_element))
                      (set `self.KnockBackDirection` (- (`self.K2_GetActorLocation` _array_element) (`self.K2_GetActorLocation`)))
                      (`AuraAbilitySystemLibrary.SetKnockBackDirection` _explosiondamageparams (`KismetMathLibrary.GetForwardVector` (`KismetMathLibrary.MakeRotator` _returnvalue_roll 45.0 _returnvalue_yaw)) 600.0)
                      (`AuraAbilitySystemLibrary.SetDeathImpulseDirection` _explosiondamageparams (`self.KnockBackDirection`) 600.0)
                      (`AuraAbilitySystemLibrary.ApplyDamageEffect` (`self.ExplosionDamageParams`)))
                    (`self.K2_DestroyActor`)))))
            (:`else`)))))))

(fn `IsWithingDistance`
  (returns (ReturnValue :type Boolean))
  (return (<= (`KismetMathLibrary.VSize` (- (`self.K2_GetActorLocation`) (`self.K2_GetActorLocation` (`self.ReturnToActor`)))) (`self.ExplodeDistance`))))

(fn `UserConstructionScript`)